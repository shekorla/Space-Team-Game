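; Enemy bullet projectile Blueprint for a side-scroller that damages what it strikes and destroys itself one second after spawning.
; A hit applies Damage to any struck actor and destroys the bullet, as does a projectile movement bounce, without damage.
; A Sphere overlap damages only a SideScrollerCharacter and leaves the bullet alive.
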(event `self.ReceiveBeginPlay`
  ;[1 1 1] Start
  (`KismetSystemLibrary.Delay` 1.0)
  (`self.K2_DestroyActor`))

(event `self.ReceiveHit`
  (params (MyComp :type "PrimitiveComponent Object Reference") (Other :type "Actor Object Reference") (OtherComp :type "PrimitiveComponent Object Reference") (bSelfMoved :type Boolean) (HitLocation :type "Vector Structure") (HitNormal :type "Vector Structure") (NormalImpulse :type "Vector Structure") (Hit :type "HitResult Structure (by ref)"))
  ;[1 1 1] When Bullet Hits Player
  (`GameplayStatics.ApplyDamage` Other (`self.Damage`) null self)
  (`self.K2_DestroyActor`))

(event `self.Sphere.OnComponentBeginOverlap`
  (params (OverlappedComponent :type "PrimitiveComponent Object Reference") (OtherActor :type "Actor Object Reference") (OtherComp :type "PrimitiveComponent Object Reference") (OtherBodyIndex :type Integer) (bFromSweep :type Boolean) (SweepResult :type "HitResult Structure (by ref)"))
  ;[1 1 1] Apply Damage
  (bind _asside_scroller_character (cast `/Game/SideScrollerBP/Blueprints/SideScrollerCharacter` OtherActor))
  (`GameplayStatics.ApplyDamage` _asside_scroller_character (`self.Damage`)))

(event `self.ProjectileMovement.OnProjectileBounce`
  (params (ImpactResult :type "HitResult Structure (by ref)") (ImpactVelocity :type "Vector Structure (by ref)"))
  ;[1 1 1] Destroy Bullet
  (`self.K2_DestroyActor`))

(fn `UserConstructionScript`)
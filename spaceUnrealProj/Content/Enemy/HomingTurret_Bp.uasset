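; Enemy turret that aims at the SideScrollerCharacter player and fires bullets at it.
; A Delay on Tick paces each cycle, which snaps the turret toward the player and spawns a Bullet aimed ahead using player velocity scaled by distance.
; Capsule overlap damages the player, and incoming damage lowers CurrentHealth until the turret is destroyed.
; The node setting CurrentHealth to MaxHealth is disconnected, so it never runs.
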(event `self.ReceiveBeginPlay`
  ;[1 1 1] Start
  (bind _asside_scroller_character (cast `/Game/SideScrollerBP/Blueprints/SideScrollerCharacter` (`GameplayStatics.GetPlayerPawn` 0)))
  (set `self.Player Ref` _asside_scroller_character))

(event `self.ReceiveTick`
  (params (DeltaSeconds :type "Float (single-precision)"))
  (bind _player_ref (`self.Player Ref`))
  (bind _returnvalue (`SceneComponent.K2_GetComponentLocation` (`self.SpawnPoint`)))
  (bind _returnvalue_2 (`SceneComponent.K2_GetComponentLocation` (`Actor.RootComponent` _player_ref)))
  ;[1 1 1] Turret Movement
  (`KismetSystemLibrary.Delay` 1.3)
  (`self.K2_SetActorRotation` (`KismetMathLibrary.FindLookAtRotation` _returnvalue _returnvalue_2))
  (`|SpawnActorFromClass` "/Game/Enemy/Bullet.Bullet_C" (`KismetMathLibrary.MakeTransform` _returnvalue (`KismetMathLibrary.FindLookAtRotation` _returnvalue (+ _returnvalue_2 (* (`self.GetVelocity` _player_ref) (/ (`self.GetDistanceTo` _player_ref) 200.0))))) "AdjustIfPossibleButAlwaysSpawn" "OverrideRootScale" null null))

(event `self.Capsule.OnComponentBeginOverlap`
  (params (OverlappedComponent :type "PrimitiveComponent Object Reference") (OtherActor :type "Actor Object Reference") (OtherComp :type "PrimitiveComponent Object Reference") (OtherBodyIndex :type Integer) (bFromSweep :type Boolean) (SweepResult :type "HitResult Structure (by ref)"))
  ;[1 1 1] Apply Damage
  (bind _asside_scroller_character (cast `/Game/SideScrollerBP/Blueprints/SideScrollerCharacter` OtherActor))
  (`GameplayStatics.ApplyDamage` _asside_scroller_character (`self.Damage`)))

(event `self.ReceiveAnyDamage`
  (params (Damage :type "Float (single-precision)") (DamageType :type "DamageType Object Reference") (InstigatedBy :type "Controller Object Reference") (DamageCauser :type "Actor Object Reference"))
  ;[1 1 1] Receive Damage
  (set `self.CurrentHealth` (- (`self.CurrentHealth`) Damage))
  (if (<= (`self.CurrentHealth`) 0.0)
    (`self.K2_DestroyActor`)))

(fn `UserConstructionScript`)
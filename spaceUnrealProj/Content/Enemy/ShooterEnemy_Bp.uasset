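; Side-scroller enemy Blueprint that patrols between target points, damages the player on contact and can be killed; no shooting logic is present.
; A self-calling MoveTo event drives AI movement, pausing briefly after each successful move before advancing or resetting the target index.
; Capsule overlap with SideScrollerCharacter applies damage.
; Incoming damage lowers CurrentHealth, initialized from MaxHealth, and destroys the actor once it is depleted.
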(event `self.ReceiveBeginPlay`
  ;[1 1 1] Start
  (set `self.CurrentHealth` (`self.MaxHealth`))
  (`self.MoveTo`))

(event `MoveTo`
  (`|AIMoveTo` self (0.0 0.0 0.0) (`|GetArrayItem` (`self.TargetPoints`) (`self.TargetPointIndex`))
    (:`then`
      (`KismetSystemLibrary.Delay` 1.0)
      (if (>= (- (`self.TargetPointIndex`) (`KismetArrayLibrary.Array_Length` (`self.TargetPoints`))) 0)
        (set `self.TargetPointIndex` 0)
        (else
          (`/Engine/EditorBlueprintResources/StandardMacros.IncrementInt` (`self.TargetPointIndex`)
            (:`  `
              _))))
      (`self.MoveTo`))))

(event `self.CapsuleComponent.OnComponentBeginOverlap`
  (params (OverlappedComponent :type "PrimitiveComponent Object Reference") (OtherActor :type "Actor Object Reference") (OtherComp :type "PrimitiveComponent Object Reference") (OtherBodyIndex :type Integer) (bFromSweep :type Boolean) (SweepResult :type "HitResult Structure (by ref)"))
  ;[1 1 1] Apply Damage
  (bind _asside_scroller_character (cast `/Game/SideScrollerBP/Blueprints/SideScrollerCharacter` OtherActor))
  (`GameplayStatics.ApplyDamage` _asside_scroller_character (`self.Damage`)))

(event `self.ReceiveAnyDamage`
  (params (Damage :type "Float (single-precision)") (DamageType :type "DamageType Object Reference") (InstigatedBy :type "Controller Object Reference") (DamageCauser :type "Actor Object Reference"))
  ;[1 1 1] Receive Damage
  (set `self.CurrentHealth` (- (`self.CurrentHealth`) Damage))
  (if (<= (`self.CurrentHealth`) 0.0)
    (`self.K2_DestroyActor`)))

(fn `UserConstructionScript`)
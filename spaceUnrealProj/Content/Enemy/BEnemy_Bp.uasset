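; BEnemy_Bp is a side-scroller enemy that patrols, shoots and hurts the player on contact.
; AI MoveTo cycles through TargetPoints, pausing briefly at each and continuing only when a move succeeds.
; From BeginPlay, a looping Delay spawns Bullet2_Bp at the SpawnBullet component's transform throughout, independent of any target.
; Capsule overlap with a SideScrollerCharacter applies Damage to it.
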(event `self.ReceiveBeginPlay`
  (bind _spawnbullet (`self.SpawnBullet`))
  ;[1 1 1] Start/Shoot Bullets
  (`self.Moving To`)
  (`KismetSystemLibrary.Delay` 0.5 :!label _label)
  (`|SpawnActorFromClass` "/Game/Enemy/Bullet2_Bp.Bullet2_Bp_C" (`KismetMathLibrary.MakeTransform` (`SceneComponent.K2_GetComponentLocation` _spawnbullet) (`SceneComponent.K2_GetComponentRotation` _spawnbullet)) "AdjustIfPossibleButAlwaysSpawn" "OverrideRootScale" null null)
  (goto _label))

(event `Moving To`
  ;[1 1 1] Enemy Movement
  (`|AIMoveTo` self (0.0 0.0 0.0) (`|GetArrayItem` (`self.TargetPoints`) (`self.TargetPointIndex`))
    (:`OnSuccess`
      (`KismetSystemLibrary.Delay` 1.0)
      (if (>= (`self.TargetPointIndex`) (- (`KismetArrayLibrary.Array_Length` (`self.TargetPoints`)) 1))
        (set `self.TargetPointIndex` 0)
        (else
          (`/Engine/EditorBlueprintResources/StandardMacros.IncrementInt` (`self.TargetPointIndex`)
            (:`  `
              _))))
      (`self.Moving To`))))

(event `self.CapsuleComponent.OnComponentBeginOverlap`
  (params (OverlappedComponent :type "PrimitiveComponent Object Reference") (OtherActor :type "Actor Object Reference") (OtherComp :type "PrimitiveComponent Object Reference") (OtherBodyIndex :type Integer) (bFromSweep :type Boolean) (SweepResult :type "HitResult Structure (by ref)"))
  ;[1 1 1] Apply Damage
  (bind _asside_scroller_character (cast `/Game/SideScrollerBP/Blueprints/SideScrollerCharacter` OtherActor))
  (`GameplayStatics.ApplyDamage` _asside_scroller_character (`self.Damage`)))

(fn `UserConstructionScript`)
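; Enemy that patrols a looping route of target points while firing projectiles, for what appears to be a side-scroller.
; AI MoveTo walks it to each point, pauses briefly on success, then advances the index, wrapping to the first.
; A delayed loop from BeginPlay continuously spawns Bullet2 at the SpawnBullet component, and capsule overlap with a SideScrollerCharacter triggers Apply Damage.
; Health initializes to MaxHealth but is not otherwise used here.
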(event `self.ReceiveBeginPlay`
  (bind _spawnbullet (`self.SpawnBullet`))
  ;[1 1 1] Start/Shoot
  (set `self.Health` (`self.MaxHealth`))
  (`self.MoveTo`)
  (`KismetSystemLibrary.Delay` 1.0 :!label _label)
  (`|SpawnActorFromClass` "/Game/Enemy/Bullet2.Bullet2_C" (`KismetMathLibrary.MakeTransform` (`SceneComponent.K2_GetComponentLocation` _spawnbullet) (`SceneComponent.K2_GetComponentRotation` _spawnbullet)) "AdjustIfPossibleButAlwaysSpawn" "OverrideRootScale" null null)
  (goto _label))

(event `MoveTo`
  ;[1 1 1] Movement
  (`|AIMoveTo` self (0.0 0.0 0.0) (`|GetArrayItem` (`self.TargetPoints`) (`self.TargetPointIndex`))
    (:`OnSuccess`
      (`KismetSystemLibrary.Delay` 1.0)
      (if (>= (`self.TargetPointIndex`) (- (`KismetArrayLibrary.Array_Length` (`self.TargetPoints`)) 1))
        (set `self.TargetPointIndex` 0)
        (else
          (`/Engine/EditorBlueprintResources/StandardMacros.IncrementInt` (`self.TargetPointIndex`)
            (:`  `
              _))))
      (`self.MoveTo`))))

(event `self.CapsuleComponent.OnComponentBeginOverlap`
  (params (OverlappedComponent :type "PrimitiveComponent Object Reference") (OtherActor :type "Actor Object Reference") (OtherComp :type "PrimitiveComponent Object Reference") (OtherBodyIndex :type Integer) (bFromSweep :type Boolean) (SweepResult :type "HitResult Structure (by ref)"))
  ;[1 1 1] Apply Damage
  (cast `/Game/SideScrollerBP/Blueprints/SideScrollerCharacter` OtherActor)
  (`GameplayStatics.ApplyDamage` null (`self.Damage`)))

(fn `UserConstructionScript`)